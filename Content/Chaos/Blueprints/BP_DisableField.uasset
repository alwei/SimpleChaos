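; BP_DisableField is a Chaos field actor that disables rigid bodies within a box volume when they fall below a Magnitude threshold.
; Every Tick, it applies a Disable Threshold physics field through its FieldSystemComponent.
; A box falloff supplies Magnitude with no falloff, and a culling field built from the same Box transform culls the outside, confining the effect to that volume.
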(event `self.ReceiveTick`
  (params (DeltaSeconds :type "Float (single-precision)"))
  (bind _returnvalue (`SceneComponent.K2_GetComponentToWorld` (`self.Box`)))
  ;[0.07741 0.8108 0 0.25] Disable Field
  (`FieldSystemComponent.ApplyPhysicsField` (`self.FieldSystemComponent`) true "Field_DisableThreshold" null (`CullingField.SetCullingField` (`self.CullingField`) (`BoxFalloff.SetBoxFalloff` (`self.BoxFalloff - Culling`) 1.0 0.0 1.0 0.0 _returnvalue "Field_FallOff_None") (`BoxFalloff.SetBoxFalloff` (`self.BoxFalloff`) (`self.Magnitude`) 0.0 1.0 0.0 _returnvalue "Field_FallOff_None") "Field_Culling_Outside")))

(fn `UserConstructionScript`)