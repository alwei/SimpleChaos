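; BP_ForceField is a Chaos field actor that applies strain and an outward or inward radial force to physics objects on BeginPlay.
; A radial falloff with no attenuation applies External Cluster Strain, sized and centered by SphereCol, to break clustered Geometry Collections.
; A radial vector then applies Linear Force from the FieldSystemComponent's location, with no culling to the sphere.
; StrainMagnitude and ForceMagnitude set the two strengths.
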(event `self.ReceiveBeginPlay`
  (bind _fieldsystemcomponent (`self.FieldSystemComponent`))
  (bind _spherecol (`self.SphereCol`))
  ;[0 0.1382 1 0.25] Force Field
  ;;[0.5295 0.04161 0.201 0.25] External Strain （スフィア形状の力場を発生させる）
  (`FieldSystemComponent.ApplyPhysicsField` _fieldsystemcomponent true "Field_ExternalClusterStrain" null (`RadialFalloff.SetRadialFalloff` (`self.RadialFalloff - Strain`) (`self.StrainMagnitude`) 0.0 1.0 0.0 (`SphereComponent.GetScaledSphereRadius` _spherecol) (`SceneComponent.K2_GetComponentLocation` _spherecol) "Field_FallOff_None"))
  ;;[0 0.1382 1 0.25] Linear Force （放射状にリニアな力場を発生させる）
  (`FieldSystemComponent.ApplyPhysicsField` _fieldsystemcomponent true "Field_LinearForce" null (`RadialVector.SetRadialVector` (`self.RadialVector - Force`) (`self.ForceMagnitude`) (`SceneComponent.K2_GetComponentLocation` _fieldsystemcomponent))))

(fn `UserConstructionScript`)