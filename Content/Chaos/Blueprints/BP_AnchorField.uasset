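; BP_AnchorField is a Chaos field actor that anchors physics objects within a box by setting their dynamic state to Static.
; Its construction script resets the field system, then registers a dynamic-state command built from a uniform integer, culled outside a box falloff taken from the Box component's world transform.
; It only configures the field command, running no simulation itself, and its event graph is empty.
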(fn `UserConstructionScript`
  (bind _fieldsystemcomponent (`self.FieldSystemComponent`))
  ;[1 0.6 0 0.243] Anchor Field
  ;;[1 0.6 0 0.243 20] コンストラクションスクリプト上で確実な更新のために一度フィールドを完全に削除しておく必要がある。
  (`FieldSystemComponent.ResetFieldSystem` _fieldsystemcomponent)
  ;;[1 0.6 0 0.243 20] ここでは実際の物理演算を行わずにあくまでもアンカー設定のフィールドコマンドを設定しているのみ。
  (`FieldSystemComponent.AddFieldCommand` _fieldsystemcomponent true "Field_DynamicState" null (`CullingField.SetCullingField` (`self.CullingField`) (`BoxFalloff.SetBoxFalloff` (`self.BoxFalloff`) 1.0 1.0 1.0 0.0 (`SceneComponent.K2_GetComponentToWorld` (`self.Box`)) "Field_FallOff_None") (`UniformInteger.SetUniformInteger` (`self.UniformInteger`) (`KismetMathLibrary.Conv_ByteToInt` (`self.Static`))) "Field_Culling_Outside")))